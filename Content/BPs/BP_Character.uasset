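; BP_Character is a character Blueprint that performs the interactions offered by its assigned building.
; ProcessInteraction constructs an object from each class in the building's Interactions list, passing itself as context, then stores it and calls Interact.
; StopInteraction stops every stored interaction object and clears the list.
; The event graph and construction script are empty, so both functions depend on external callers.
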(fn `ProcessInteraction`
  (for _array_element (`/Game/BPs/BP_Building.Interactions` (`self.AssignedBuilding`))
    (bind _returnvalue (`|GenericCreateObject` _array_element self))
    (`KismetArrayLibrary.Array_Add` (`self.CurrentInteractions`) _returnvalue)
    (`/Game/BPs/Interaction/InteractionScript.Interact` _returnvalue)))

(fn `StopInteraction`
  (for _array_element (`self.CurrentInteractions`)
    (`/Game/BPs/Interaction/InteractionScript.Stop Interaction` _array_element))
  (`KismetArrayLibrary.Array_Clear` (`self.CurrentInteractions`)))

(fn `UserConstructionScript`)